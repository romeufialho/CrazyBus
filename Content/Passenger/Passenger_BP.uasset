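; Passenger actor that idles until a TestVehicle_BP enters its DetectionSphere, then plays a run animation and destroys itself one second later.
; While targeted it moves every Tick; MoveTowardsTarget applies the normalized vehicle-to-passenger direction as a local offset, despite its name.
; Leaving the detection sphere clears the target, and vehicle contact with the DestructionSphere destroys the passenger immediately.
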(event OnComponentBeginOverlap(DetectionSphere)
  (params (OverlappedComponent :type Primitive%20Component%20Object%20Reference) (OtherActor :type Actor%20Object%20Reference) (OtherComp :type Primitive%20Component%20Object%20Reference) (OtherBodyIndex :type Integer) (bFromSweep :type Boolean) (SweepResult :type Hit%20Result%20Structure%20%28by%20ref%29))
  (bind _astest_vehicle_bp (Utilities|Casting|CastToTestVehicle_BP OtherActor))
  (Utilities|IsValid _astest_vehicle_bp
    (:Is%20Valid
      (Variables|Default|SetTargetActor _astest_vehicle_bp)
      (Utilities|FlowControl|Sequence
        (:then_0
          (Components|Animation|PlayAnimation (Variables|Character|GetMesh) "/Game/Passenger/Passenger_Run.Passenger_Run" true))
        (:then_1
          (Utilities|FlowControl|Delay 1.0)
          (CallFunction|Destroy))))))

(event OnComponentEndOverlap(DetectionSphere)
  (params (OverlappedComponent :type Primitive%20Component%20Object%20Reference) (OtherActor :type Actor%20Object%20Reference) (OtherComp :type Primitive%20Component%20Object%20Reference) (OtherBodyIndex :type Integer))
  (bind _astest_vehicle_bp (Utilities|Casting|CastToTestVehicle_BP OtherActor))
  (Utilities|IsValid _astest_vehicle_bp
    (:Is%20Valid
      (Variables|Default|SetTargetActor 0))))

(event OnComponentBeginOverlap(DestructionSphere)
  (params (OverlappedComponent :type Primitive%20Component%20Object%20Reference) (OtherActor :type Actor%20Object%20Reference) (OtherComp :type Primitive%20Component%20Object%20Reference) (OtherBodyIndex :type Integer) (bFromSweep :type Boolean) (SweepResult :type Hit%20Result%20Structure%20%28by%20ref%29))
  (bind _astest_vehicle_bp (Utilities|Casting|CastToTestVehicle_BP OtherActor))
  (Utilities|IsValid _astest_vehicle_bp
    (:Is%20Valid
      (Variables|Default|SetTargetActor _astest_vehicle_bp)
      (Actor|DestroyActor))))

(event Custom|MoveTowardsTarget
  (Transformation|AddActorLocalOffset (* (Math|Vector|Normalize (- (Transformation|GetActorLocation) (Transformation|GetActorLocation (Variables|Default|GetTargetActor)))) (Utilities|Time|GetWorldDeltaSeconds) (Variables|Default|GetSpeed)) false false))

(event Custom|Destroy
  (Actor|DestroyActor))

(event EventBeginPlay
  (Components|Animation|PlayAnimation (Variables|Character|GetMesh) "/Game/Passenger/Passenger_Idle.Passenger_Idle" false))

(event Collision|EventActorBeginOverlap
  (params (OtherActor :type Actor%20Object%20Reference)))

(event EventTick
  (params (DeltaSeconds :type Float%20%28single-precision%29))
  (Variables|Default|GetTargetActor
    (:then
      (CallFunction|MoveTowardsTarget))
    (:else)))

(fn ConstructionScript)