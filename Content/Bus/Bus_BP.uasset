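; Bus_BP is a player-drivable bus that uses a vehicle movement component and a spring arm camera.
; Every tick it polls Enhanced Input action values and passes throttle, brake, steering and handbrake to the movement component.
; The look-around input adds yaw to the spring arm each tick, without scaling by delta time.
; The IA_Throttle event is empty, and a leftover throttle call in the event graph never runs.
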(event Input|EnhancedActionEvents|EnhancedInputActionIA_Throttle
  (params (ActionValue :type Float%20%28double-precision%29) (ElapsedSeconds :type Float%20%28double-precision%29) (TriggeredSeconds :type Float%20%28double-precision%29) (InputAction :type Input%20Action%20Object%20Reference :default "/Game/VehicleTemplate/Input/Actions/IA_Throttle.IA_Throttle")))

(event EventTick
  (params (DeltaSeconds :type Float%20%28single-precision%29))
  (CallFunction|VehicleInput)
  (CallFunction|CameraInput))

(fn ConstructionScript)

(fn VehicleInput
  (bind _vehiclemovementcomponent (Variables|Default|GetVehicleMovementComponent))
  (Class|ChaosVehicleMovementComponent|SetThrottleInput _vehiclemovementcomponent (Input|EnhancedActionValues|GetIA_Throttle))
  (Class|ChaosVehicleMovementComponent|SetBrakeInput _vehiclemovementcomponent (Input|EnhancedActionValues|GetIA_Brake))
  (Class|ChaosVehicleMovementComponent|SetSteeringInput _vehiclemovementcomponent (Input|EnhancedActionValues|GetIA_Steering))
  (Class|ChaosVehicleMovementComponent|SetHandbrakeInput _vehiclemovementcomponent (Input|EnhancedActionValues|GetIA_Handbrake)))

(fn CameraInput
  (Transformation|AddRelativeRotation (Variables|Default|GetSpringArm) (Math|Rotator|MakeRotator 0.0 0.0 (Input|EnhancedActionValues|GetIA_LookAround)) false false))