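; Bus_BP is the drivable bus vehicle, with an orbiting camera and an arrow that points toward a bus stop.
; Each Tick it feeds Enhanced Input values for throttle, brake, steering and handbrake into the vehicle movement component.
; Look-around input yaws the spring arm.
; The arrow mesh eases its world yaw toward the BusStopPlaceHolder actor using RInterpTo on a look-at rotation.
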(event EventBeginPlay)

(event EventTick
  (params (DeltaSeconds :type Float%20%28single-precision%29))
  (CallFunction|VehicleInput)
  (CallFunction|CameraInput)
  (CallFunction|RotateDirectionalArrow))

(fn ConstructionScript)

(fn VehicleInput
  (bind _vehiclemovementcomponent (Variables|Default|GetVehicleMovementComponent))
  (Class|ChaosVehicleMovementComponent|SetThrottleInput _vehiclemovementcomponent (Input|EnhancedActionValues|GetIA_Throttle))
  (Class|ChaosVehicleMovementComponent|SetBrakeInput _vehiclemovementcomponent (Input|EnhancedActionValues|GetIA_Brake))
  (Class|ChaosVehicleMovementComponent|SetSteeringInput _vehiclemovementcomponent (Input|EnhancedActionValues|GetIA_Steering))
  (Class|ChaosVehicleMovementComponent|SetHandbrakeInput _vehiclemovementcomponent (Input|EnhancedActionValues|GetIA_Handbrake)))

(fn CameraInput
  (Transformation|AddRelativeRotation (Variables|Default|GetSpringArm) (Math|Rotator|MakeRotator 0.0 0.0 (Input|EnhancedActionValues|GetIA_LookAround)) false false))

(fn RotateDirectionalArrow
  (bind _arrow_mesh (Variables|Default|GetArrow%20Mesh))
  (Transformation|SetWorldRotation _arrow_mesh (Math|Rotator|MakeRotator 0.0 0.0 (.yaw (Math|Interpolation|RInterpTo (Transformation|GetWorldRotation _arrow_mesh) (Math|Rotator|FindLookatRotation (Transformation|GetWorldLocation _arrow_mesh) (Transformation|GetActorLocation (Variables|Default|GetBusStopPlaceHolder))) (Utilities|Time|GetWorldDeltaSeconds) 1.0))) false false))