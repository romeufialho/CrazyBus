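; MyVehicle_BP is a test vehicle Blueprint that the player drives through input actions.
; Each Tick, it reads the throttle, brake, steering and handbrake action values and passes them straight to the vehicle movement component.
; The look-around action value is added as yaw to the spring arm every frame, without delta-time scaling.
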(event EventBeginPlay)

(event Collision|EventActorBeginOverlap
  (params (OtherActor :type Actor%20Object%20Reference)))

(event EventTick
  (params (DeltaSeconds :type Float%20%28single-precision%29))
  (bind _vehiclemovementcomponent (Variables|Default|GetVehicleMovementComponent))
  (Class|ChaosVehicleMovementComponent|SetThrottleInput _vehiclemovementcomponent (Input|EnhancedActionValues|GetIA_Throttle))
  (Class|ChaosVehicleMovementComponent|SetBrakeInput _vehiclemovementcomponent (Input|EnhancedActionValues|GetIA_Brake))
  (Class|ChaosVehicleMovementComponent|SetSteeringInput _vehiclemovementcomponent (Input|EnhancedActionValues|GetIA_Steering))
  (Class|ChaosVehicleMovementComponent|SetHandbrakeInput _vehiclemovementcomponent (Input|EnhancedActionValues|GetIA_Handbrake))
  (Transformation|AddRelativeRotation (Variables|Default|GetSpringArm) (Math|Rotator|MakeRotator 0.0 0.0 (Input|EnhancedActionValues|GetIA_LookAround)) false false))

(fn ConstructionScript)