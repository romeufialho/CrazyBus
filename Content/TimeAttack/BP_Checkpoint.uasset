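; BP_Checkpoint is a bus stop checkpoint for the time attack mode that awards time when the player reaches it while it is targeted.
; On player overlap with its trigger box, a targeted stop restores the normal material on its two cubes and clears its targeted flag.
; It then passes passenger count times a time multiplier to GM_TimeAttack1 as time to add.
; Untargeted stops only print a message, and two dispatcher calls sit unused.
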(event OnComponentBeginOverlap(TriggerBox)
  (params (OverlappedComponent :type Primitive%20Component%20Object%20Reference) (OtherActor :type Actor%20Object%20Reference) (OtherComp :type Primitive%20Component%20Object%20Reference) (OtherBodyIndex :type Integer) (bFromSweep :type Boolean) (SweepResult :type Hit%20Result%20Structure%20%28by%20ref%29))
  (if (== OtherActor (Game|Player|GetPlayerPawn 0))
    (if (Variables|Default|GetisBusStopTargeted)
      (Rendering|Material|SetMaterial (Variables|Default|GetCube) 0 "/Game/TimeAttack/Mat_Normal.Mat_Normal")
      (Variables|Default|SetisBusStopTargeted false)
      (Development|PrintString (Utilities|String|Append "Removed: " (Utilities|GetDisplayName self)))
      (bind _asgm_time_attack_1 (Utilities|Casting|CastToGM_TimeAttack1 (Game|GetGameMode)))
      (bind _output_get (Variables|Default|SetTimeToAdd (* (Variables|Default|GetPassengerNum) (Variables|Default|GetTimeMultiplier))))
      (Default|ChekpointCrossed _asgm_time_attack_1 _output_get)
      (else
        (Development|PrintString "Checkpoint not Valid!")))))

(fn ConstructionScript)